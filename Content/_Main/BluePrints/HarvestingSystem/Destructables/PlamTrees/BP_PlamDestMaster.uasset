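; Base Blueprint for palm tree destructibles in the harvesting system, which dissolves the palm away some seconds after it spawns.
; After the parent BeginPlay and a fixed delay, it creates dynamic material instances for the static mesh's trunk and leaf material slots.
; A timeline drives their Dissolve parameter, then hides the mesh on finish without destroying the actor.
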(event EventBeginPlay
  (|CallParentFunction) ; 需要调用父类的设置
  (Utilities|FlowControl|Delay 7.0)
  (bind _returnvalue (Rendering|Material|CreateDynamicMaterialInstance (Variables|Default|GetStaticMesh) 0 "/Game/_Main/Meshes/PalmTrees/Material/M_Palm01.M_Palm01" "None" :!class /Script/Engine.PrimitiveComponent))
  (Variables|Default|SetMat0 _returnvalue)
  (bind _returnvalue_2 (Rendering|Material|CreateDynamicMaterialInstance (Variables|Default|GetStaticMesh) 1 "/Game/_Main/Meshes/PalmTrees/Material/M_Palm02.M_Palm02" "None" :!class /Script/Engine.PrimitiveComponent))
  (Variables|Default|SetMat1 _returnvalue_2)
  (bind _returnvalue_3 (Rendering|Material|CreateDynamicMaterialInstance (Variables|Default|GetStaticMesh) 2 "/Game/_Main/Meshes/PalmTrees/Material/M_Palm03.M_Palm03" "None" :!class /Script/Engine.PrimitiveComponent))
  (Variables|Default|SetMat2 _returnvalue_3)
  (bind _returnvalue_4 (Rendering|Material|CreateDynamicMaterialInstance (Variables|Default|GetStaticMesh) 3 "/Game/_Main/Meshes/PalmTrees/Material/M_Palm03.M_Palm03" "None" :!class /Script/Engine.PrimitiveComponent))
  (Variables|Default|SetMat3 _returnvalue_4)
  (bind _returnvalue_5 (Rendering|Material|CreateDynamicMaterialInstance (Variables|Default|GetStaticMesh) 4 "/Game/_Main/Meshes/PalmTrees/Material/M_PalmLeaf_Inst.M_PalmLeaf_Inst" "None" :!class /Script/Engine.PrimitiveComponent))
  (Variables|Default|SetMat4 _returnvalue_5)
  (bind _returnvalue_6 (Rendering|Material|CreateDynamicMaterialInstance (Variables|Default|GetStaticMesh) 5 "/Game/_Main/Meshes/PalmTrees/Material/M_Palm04.M_Palm04" "None" :!class /Script/Engine.PrimitiveComponent))
  (Variables|Default|SetMat5 _returnvalue_6)
  (bind _新建轨道_0 (Timeline|FadeAwayTimeLIne PlayFromStart) ; 时间：0-1
    (:Update
      (Rendering|Material|SetScalarParameterValue (Variables|Default|GetMat0) "Dissolve" _新建轨道_0 :!class /Script/Engine.MaterialInstanceDynamic))
    (:Finished
      (Rendering|SetVisibility (Variables|Default|GetStaticMesh) false false))))

(fn ConstructionScript
  (|CallParentFunction))