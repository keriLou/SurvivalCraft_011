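; BP_DestructableTree is a physics tree piece for the harvesting system, likely spawned when a tree is felled.
; On BeginPlay it pushes its capsule with an acceleration-change force along Direction scaled by Force, then destroys itself after a fixed delay.
; An authority switch on BeginPlay does nothing; a comment says the push is meant to run on both server and clients.
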(event EventBeginPlay
  (Networking|SwitchHasAuthority ; 权限开关(远程和授权)
    (:Authority
      _)
    (:Remote
      _))
  (CallFunction|AddForce) ; 该函数将被调用在服务器和客户端
  (Utilities|FlowControl|Delay 15.0)
  (Actor|DestroyActor))

(fn ConstructionScript
  (|CallParentFunction))

(fn AddForce
  (Physics|AddForce (Variables|Default|GetCapsule) (* (Variables|Default|GetDirection) (LocalVariables|GetForce)) "None" true))