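; Survival game player controller that owns the client-side HUD and relays inventory changes to it.
; On non-authority instances it creates the main widget at BeginPlay; Tab or I toggles the inventory, cursor and input mode.
; Slot update and reset events find the slot widget by container and index, with only inventory and hotbar grids wired, not storage or armor.
; A further event forwards collected-item notifications to the main widget.
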(event Custom|InventoryOnClient
  (if (Variables|Default|GetInventoryShown?)
    (Default|SetInventoryVis (Variables|Default|GetMainWidgetRef) false)
    (Variables|Default|SetbShowMouseCursor false)
    (Input|SetInputModeGameOnly self)
    (Variables|Default|SetInventoryShown? false)
    (else
      (Default|SetInventoryVis (Variables|Default|GetMainWidgetRef) true)
      (Variables|Default|SetbShowMouseCursor true)
      (Input|SetInputModeGameandUI self 0 "DoNotLock" true)
      (Variables|Default|SetInventoryShown? true))))

(event Custom|ResetItemSlot
  (params (Container :type E_ContainerType%20Enum :default "NewEnumerator0") (Index :type Integer))
  (bind _widget (CallFunction|GetIneventoryWidget Container Index))
  (Utilities|IsValid _widget
    (:Is%20Valid
      (Default|ResetSlot _widget))))

(event Custom|UpdateItemSlot
  (params (Container :type E_ContainerType%20Enum :default "NewEnumerator0") (Index :type Integer) (ItemInfo :type S%20Item%20Info%20Structure))
  (bind _widget (CallFunction|GetIneventoryWidget Container Index))
  (Utilities|IsValid _widget
    (:Is%20Valid
      (Default|UpdateSlot _widget ItemInfo))))

(event Custom|ShowItemWidget
  (params (ResourceImage :type Texture%202D%20Object%20Reference) (ResourceQuantiry :type Integer) (ResourceName :type Text))
  (Default|ShowItemCollected (Variables|Default|GetMainWidgetRef) ResourceImage ResourceQuantiry ResourceName))

(event EventBeginPlay
  ;[0.1677 0.1677 0.1677] 将主控件（W_MainWeiget）添加到客户端视口
  ;;[1 1 1] Authority 在服务器执行；Remote在客户端执行
  (Networking|SwitchHasAuthority ; 开关权限
    (:Remote
      (bind _returnvalue (UserInterface|CreateWidget "/Game/_Main/Widgets/W_MainWidget.W_MainWidget_C" self)) ; create widget
      (bind _output_get (Variables|Default|SetMainWidgetRef _returnvalue))
      (UserInterface|Viewport|AddtoViewport _output_get 0))))

(event Input|KeyboardEvents|Tab
  (params (Key :type Key%20Structure :default "None"))
  ;[0.1219 0.1219 0.1219] 按键控制 库存 在 客户端 的显隐
  (:Pressed
    (CallFunction|InventoryonClient)))

(event Input|KeyboardEvents|I
  (params (Key :type Key%20Structure :default "None"))
  ;[0.1219 0.1219 0.1219] 按键控制 库存 在 客户端 的显隐
  (:Pressed
    (CallFunction|InventoryonClient)))

(fn ConstructionScript)

(fn GetIneventoryWidget
  (params (Container :type E_ContainerType%20Enum :default "NewEnumerator0") (SlotIndex :type Integer))
  (return (Utilities|Array|Get(acopy) (Variables|/Game/_Main/Widgets/InventoryWidgets/W_ItemContainerGrid.W_ItemContainerGrid_C|GetSlots (Utilities|Select :Index Container :NewEnumerator0 (Variables|/Game/_Main/Widgets/InventoryWidgets/W_Inventory.W_Inventory_C|GetW_ItemContainerGrid (Variables|/Game/_Main/Widgets/W_MainWidget.W_MainWidget_C|GetW_Inventory (Variables|Default|GetMainWidgetRef))) :NewEnumerator1 (Variables|/Game/_Main/Widgets/InventoryWidgets/W_Hotbar.W_Hotbar_C|GetW_ItemContainerGrid (Variables|/Game/_Main/Widgets/W_MainWidget.W_MainWidget_C|GetW_Hotbar (Variables|Default|GetMainWidgetRef))) :NewEnumerator2 0 :NewEnumerator3 0)) SlotIndex)))

(fn SurvivalGamePCRef
  (return self))