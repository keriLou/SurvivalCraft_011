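; Equippable hatchet tool that chops large harvestable items such as trees for resources.
; Using it plays first- and third-person montages, and a notify triggers a debug-drawn sphere overlap at the owner's arrow location.
; HarvestFoliage subtracts health; surviving hits grant data-table resources scaled by preferred tool, tier, damage and randomness.
; At zero health it swaps the item for its data-table destruct class, passing the character's forward direction.
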(event Custom|GetRotationClient
  (bind _location (Class|BPISurvivalCharacter|GetArrowLocation(Message) (Components|GetOwner)))
  (CallFunction|ServerOverlap _location))

(event Custom|ServerOverlap
  (params (SpherePos :type Vector))
  (bind (_outactors _returnvalue) (Collision|SphereOverlapActors SpherePos 6e+01 (Utilities|Array|MakeArray "ObjectTypeQuery8") 0 (Utilities|Array|MakeArray (Variables|Default|GetChar%20Ref))))
  (Rendering|Debug|DrawDebugSphere SpherePos 6e+01 12 "(R=1.000000,G=0.000000,B=0.026565,A=1.000000)" 5.0 5.0)
  (if _returnvalue
    (for _array_element _outactors
      (CallFunction|HarvestFoliage 15.0 _array_element))
    (else
      (Development|PrintString "false"))))

(event EventBeginPlay
  (|CallParentFunction) ; 此节点被禁用，将不会被调用。\n从引脚连出引线来编译功能。
)

(event Collision|EventActorBeginOverlap
  (params (OtherActor :type Actor%20Object%20Reference))
  (|CallParentFunction OtherActor) ; 此节点被禁用，将不会被调用。\n从引脚连出引线来编译功能。
)

(event EventTick
  (params (DeltaSeconds :type Float%20%28single-precision%29))
  (|CallParentFunction DeltaSeconds) ; 此节点被禁用，将不会被调用。\n从引脚连出引线来编译功能。
)

(event EventUseItemInterface
  (params (CharRef :type BP%20First%20Person%20Character%20Object%20Reference))
  (if (not (Variables|Default|GetIsSwinging?))
    (Variables|Default|SetIsSwinging? true)
    (bind _output_get (Variables|Default|SetChar%20Ref CharRef))
    (Class|BPISurvivalCharacter|FirstPersonMontage(Message) _output_get "/Game/Man/Animations/Hatchet_Chop_Montage.Hatchet_Chop_Montage")
    (Default|ThirdPersonMontage _output_get "/Game/Man/Animations/Hatchet_Chop_Montage.Hatchet_Chop_Montage")))

(event EventNotifyInterface
  (CallFunction|GetRotationClient))

(event EventEndAnimation
  (Variables|Default|SetIsSwinging? false))

(fn ConstructionScript
  (|CallParentFunction))

(fn HarvestFoliage
  (params (Damage :type Float%20%28double-precision%29) (Ref :type Actor%20Object%20Reference))
  (LocalVariables|SetLocalDamage Damage)
  (bind _ref (Class|BPILargeItem|GetLargeItemRef(Message) Ref)) ; 得到 大物品的引用
  (Utilities|IsValid _ref ; 判断引用有效
    (:Is%20Valid
      (LocalVariables|SetLocalHealth (- (Variables|/Game/_Main/BluePrints/HarvestingSystem/BP_LargeItemMaster.BP_LargeItemMaster_C|GetHealth _ref) (LocalVariables|GetLocalDamage))) ; 得到砍伐树木后的血
      (if (<= (LocalVariables|GetLocalHealth) 0.0) ; 判断树木血量
        (bind _returnvalue (Utilities|GetDataTableRow "/Game/_Main/BluePrints/DataTypes/DT_LargeItemResources.DT_LargeItemResources" (Utilities|String|StringToName (Utilities|GetClassDisplayName (Utilities|GetClass _ref))))
          (:then
            (LocalVariables|SetLocalDestructClass (.Class (Utilities|Struct|BreakS_LargeItem _returnvalue)))
            (LocalVariables|SetLocalTransform (Transformation|GetActorTransform _ref))
            (Actor|DestroyActor _ref)
            (Game|SpawnActorfromClass (LocalVariables|GetLocalDestructClass) (LocalVariables|GetLocalTransform) "Undefined" 0 (Transformation|GetActorForwardVector (Variables|Default|GetChar%20Ref)) 0)))
        (else
          (Variables|/Game/_Main/BluePrints/HarvestingSystem/BP_LargeItemMaster.BP_LargeItemMaster_C|SetHealth _ref (LocalVariables|GetLocalHealth))
          (bind _returnvalue_2 (Utilities|GetDataTableRow "/Game/_Main/BluePrints/DataTypes/DT_LargeItemResources.DT_LargeItemResources" (Utilities|String|StringToName (Utilities|GetClassDisplayName (Utilities|GetClass _ref)))) ; 通过类名来找树的类型
            (:then
              ;[1 1 1] 砍伐过程中，得到的资源数量
              (LocalVariables|SetGivenResources (.GivenItems (Utilities|Struct|BreakS_LargeItem _returnvalue_2)))
              (for _array_element (LocalVariables|GetGivenResources)
                (LocalVariables|SetLocalResourceQuanity (Math|Float|Truncate (|((((BaseVar*RateVar)*ToolTypeVar)*ToolTierVar)*DamageVar) (Math|Conversions|ToFloat(Integer) (.Quantity (Utilities|Struct|BreakS_ResourseStructure _array_element))) 1.0 (Math|Float|SelectFloat (Math|Random|RandomFloatinRange 0.2 0.4) (Math|Random|RandomFloatinRange 0.01 0.1) (Utilities|Enum|Equal(Enum) (.PrefferedToolType (Utilities|Struct|BreakS_ResourseStructure _array_element)) (Variables|Default|GetToolType))) (Utilities|Select :Index (Variables|Default|GetToolTier) :NewEnumerator0 (Math|Random|RandomFloatinRange 0.8 1.2) :NewEnumerator1 (Math|Random|RandomFloatinRange 1.2 1.6)) (LocalVariables|GetLocalDamage))))
                (if (not (<= (LocalVariables|GetLocalResourceQuanity) 0))
                  (bind _survivalcharref (Default|GetSurvivalCharRef (Variables|Default|GetChar%20Ref)))
                  (Default|HarvestItemonServer _survivalcharref (Utilities|Struct|MakeS_ResourseStructure (.Resource (Utilities|Struct|BreakS_ResourseStructure _array_element)) (LocalVariables|GetLocalResourceQuanity) "NewEnumerator0")))))))))))