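; Player hotbar component, a child item container that holds the quick-slot items and syncs them to the UI and character.
; CheckHotbar reports whether a slot holds an item and its type.
; Drops from the player inventory or hotbar transfer the item into the target slot.
; Add and remove overrides run the parent logic, then update the controller's slot via owner messages; removal also asks the survival character to dequip that index.
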(event EventBeginPlay)

(event EventTick
  (params (DeltaSeconds :type Float%20%28single-precision%29)))

(fn CheckHotbar
  (params (Index :type Integer))
  (bind _items (Variables|Default|GetItems))
  (bind _output (Utilities|Array|Get(acopy) _items Index))
  (bind (_itemid _itemquantity _itemidicon _itemname _itemdesc _itemdamage _itemrarity _itemcurhp _itemmaxhp _isstackable_ _stacksize _itemtype) (Utilities|Struct|BreakS_ItemInfo _output))
  (if (== _itemid 0)
    (return false "NewEnumerator0")
    (else
      (return true _itemtype))))

(fn HandleSlotDrop
  (params (FromContainer :type BPC%20Items%20Container%20Object%20Reference) (FromIndex :type Integer) (DroppedIndex :type Integer))
  ;[1 1 1] 处理槽的放下1
  (LocalVariables|SetLocalFromContainer FromContainer)
  (LocalVariables|SetLocalFromIndex FromIndex)
  (LocalVariables|SetLocalDroppedIndex DroppedIndex)
  (switch Utilities|FlowControl|Switch|SwitchonE_ContainerType (Variables|/Game/_Main/BluePrints/Inventory/BPC_ItemsContainer.BPC_ItemsContainer_C|GetContainerType (LocalVariables|GetLocalFromContainer))
    (:NewEnumerator0
      _)
    (:NewEnumerator1
      _))
  (Default|TransformItem (LocalVariables|GetLocalFromContainer) self (LocalVariables|GetLocalDroppedIndex) (LocalVariables|GetLocalFromIndex))
  (return))

(fn AddItemtoIndex
  (params (Item :type S%20Item%20Info%20Structure) (LocalSpecificIndex :type Integer) (FromIndex :type Integer))
  ;[1 1 1] 将物品添加到索引2
  (bind _success_ (|CallParentFunction Item LocalSpecificIndex FromIndex))
  (bind _controllerref (Class|BPISurvivalCharacter|GetControllerfromChar(Message) (Components|GetOwner)))
  (Default|UpdateItemSlot _controllerref (Variables|Default|GetContainerType) LocalSpecificIndex (CallFunction|GetItematIndex LocalSpecificIndex))
  (return _success_))

(fn RemoveItematIndex
  (params (Index :type Integer))
  ;[1 1 1] 删除索引中的项目3
  (bind _success_ (|CallParentFunction Index))
  (bind _controllerref (Class|BPISurvivalCharacter|GetControllerfromChar(Message) (Components|GetOwner)))
  (Default|ResetItemSlot _controllerref (Variables|Default|GetContainerType) Index)
  (bind _survivalcharref (Class|BPISurvivalCharacter|GetSurvivalCharRef(Message) (Components|GetOwner)))
  (Default|DequipCurrentItem _survivalcharref Index) ; 物品不在当前快捷栏时，解除装备
  (return _success_))